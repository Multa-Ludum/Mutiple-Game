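; AI_Character is an endless runner character that moves forward automatically along its control yaw each tick until IsDead.
; TurnCorner smoothly interpolates player controller 0's rotation toward DesiredRotaion.
; The MoveRight axis adds sideways movement along the fixed world right vector, not relative to heading.
; Logic that would turn DesiredRotaion 90 degrees left or right and clear CanTurn is disconnected, so never runs.
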(event `self.ReceiveTick`
  (params (DeltaSeconds :type "Float (single-precision)"))
  (if (not (`self.IsDead`))
    (`self.TurnCorner`)
    (`self.AddMovementInput` (`KismetMathLibrary.GetForwardVector` (`KismetMathLibrary.MakeRotator` 0.0 0.0 (.yaw (`self.GetControlRotation`)))))))

(event `InputAxis|MoveRight` :overrideparent false
  (params (AxisValue :type "Float (single-precision)"))
  (`self.AddMovementInput` (`KismetMathLibrary.GetRightVector` (struct)) AxisValue))

(event `TurnCorner`
  (bind _returnvalue (`self.GetControlRotation`))
  (bind _desiredrotaion (`self.DesiredRotaion`))
  (if (!= _returnvalue _desiredrotaion)
    (`Controller.SetControlRotation` (`GameplayStatics.GetPlayerController` 0) (`KismetMathLibrary.RInterpTo` _returnvalue _desiredrotaion (`GameplayStatics.GetWorldDeltaSeconds`) 10.0))))

(fn `UserConstructionScript`)