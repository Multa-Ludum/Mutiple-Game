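; Left-corner floor tile for an endless runner that lets the player turn and can kill them on wall contact.
; Overlapping the TurnZone sets CanTurn on the RunCharacter.
; Hits on either of the two walls compare the hit normal with the character's forward vector by dot product, calling Death unless the normal almost exactly opposes that vector.
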(event `self.TurnZone.OnComponentBeginOverlap`
  (params (OverlappedComponent :type "PrimitiveComponent Object Reference") (OtherActor :type "Actor Object Reference") (OtherComp :type "PrimitiveComponent Object Reference") (OtherBodyIndex :type Integer) (bFromSweep :type Boolean) (SweepResult :type "HitResult Structure (by ref)"))
  (bind _asrun_character (cast `/Game/EndlessRunner/Blueprints/RunCharacter` OtherActor))
  (set `/Game/EndlessRunner/Blueprints/RunCharacter.CanTurn` true _asrun_character))

(event `self.Wall.OnComponentHit`
  (params (HitComponent :type "PrimitiveComponent Object Reference") (OtherActor :type "Actor Object Reference") (OtherComp :type "PrimitiveComponent Object Reference") (NormalImpulse :type "Vector Structure") (Hit :type "HitResult Structure (by ref)"))
  (bind _asrun_character (cast `/Game/EndlessRunner/Blueprints/RunCharacter` OtherActor))
  (if (not (`KismetMathLibrary.NearlyEqual_FloatFloat` (`KismetMathLibrary.Dot_VectorVector` Hit_Normal (`self.GetActorForwardVector` _asrun_character)) -1.0 0.01))
    (`/Game/EndlessRunner/Blueprints/RunCharacter.Death` _asrun_character)))

(event `self.Wall2.OnComponentHit`
  (params (HitComponent :type "PrimitiveComponent Object Reference") (OtherActor :type "Actor Object Reference") (OtherComp :type "PrimitiveComponent Object Reference") (NormalImpulse :type "Vector Structure") (Hit :type "HitResult Structure (by ref)"))
  (bind _asrun_character (cast `/Game/EndlessRunner/Blueprints/RunCharacter` OtherActor))
  (if (not (`KismetMathLibrary.NearlyEqual_FloatFloat` (`KismetMathLibrary.Dot_VectorVector` Hit_Normal (`self.GetActorForwardVector` _asrun_character)) -1.0 0.01))
    (`/Game/EndlessRunner/Blueprints/RunCharacter.Death` _asrun_character)))

(fn `UserConstructionScript`)