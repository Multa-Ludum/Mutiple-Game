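; Game mode for an endless runner that procedurally builds the track and puts a widget on screen at begin play.
; On start it spawns an initial run of ten floor pieces through AddFloorTile.
; Each piece is picked at random from straight or curve arrays and chained at the previous tile's attach transform via NextSpawnPoint.
; After eight consecutive straights, AddFloorTile inserts a random curve and resets the straight counter.
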(event `self.ReceiveBeginPlay`
  (bind _returnvalue (`|CreateWidget` null))
  (`UserWidget.AddToViewport` _returnvalue 0)
  (for _ (range 10)
    (`self.AddFloorTile` "/Game/EndlessRunner/Blueprints/BP_FloorTile.BP_FloorTile_C")))

(fn `AddFloorCurve`
  (params (Class :type "Actor Class Reference"))
  (bind _floorcurves (`self.FloorCurves`))
  (bind _returnvalue (`|SpawnActorFromClass` (`|GetArrayItem` _floorcurves (`KismetMathLibrary.RandomIntegerInRange` 0 (`KismetArrayLibrary.Array_LastIndex` _floorcurves))) (`self.NextSpawnPoint`) "Undefined" "OverrideRootScale" null null))
  (bind _asbp_floor_tile (cast `/Game/EndlessRunner/Blueprints/BP_FloorTile` _returnvalue))
  (bind _attachtransform (`/Game/EndlessRunner/Blueprints/BP_FloorTile.GetAttachTransform` _asbp_floor_tile))
  (set `self.NextSpawnPoint` _attachtransform)
  (set `self.CurrentStraights` 0))

(fn `AddFloorTile`
  (params (Class :type "Actor Class Reference"))
  (bind _floortiles (`self.FloorTiles`))
  (if (> (`self.CurrentStraights`) 7)
    (`self.AddFloorCurve` null)
    (else
      (bind _returnvalue (`|SpawnActorFromClass` (`|GetArrayItem` _floortiles (`KismetMathLibrary.RandomIntegerInRange` 0 (`KismetArrayLibrary.Array_LastIndex` _floortiles))) (`self.NextSpawnPoint`) "Undefined" "OverrideRootScale" null null))
      (bind _asbp_floor_tile (cast `/Game/EndlessRunner/Blueprints/BP_FloorTile` _returnvalue))
      (bind _attachtransform (`/Game/EndlessRunner/Blueprints/BP_FloorTile.GetAttachTransform` _asbp_floor_tile))
      (set `self.NextSpawnPoint` _attachtransform)
      (set `self.CurrentStraights` (+ (`self.CurrentStraights`) 1)))))

(fn `UserConstructionScript`)